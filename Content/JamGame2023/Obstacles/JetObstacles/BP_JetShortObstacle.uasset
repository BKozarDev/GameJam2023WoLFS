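; BP_JetShortObstacle is a short jet obstacle that penalizes the player on contact.
; It overrides the parent obstacle's Collide to cut the player's stamina by a fixed amount, run the parent logic, play a 2D bird-death sound cue and destroy itself.
; Its event graph and construction script add no behavior of their own.
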(fn `Collide`
  (params (Player :type "/Game/JamGame2023/Player/BP_PlayerChar Object Reference"))
  (`/Game/JamGame2023/Player/BP_PlayerChar.ChangeStamina` Player -15.0)
  (`parent.Collide` Player)
  (`GameplayStatics.PlaySound2D` "/Game/Audio/SC_BirdDie.SC_BirdDie" 1.0 1.0 0.0 null null)
  (`self.K2_DestroyActor`))

(fn `UserConstructionScript`
  (`parent.UserConstructionScript`))