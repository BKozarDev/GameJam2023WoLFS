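; Player-follow camera actor that tracks the character along X and plays a cinematic transition into jetpack mode.
; Each tick, while following, it snaps to a side offset, or behind and higher for one movement state.
; Jetpack events suspend following and run two timelines animating position and rotation, then resume following and add the jetpack input context.
; Setup places it offset ahead with following off; Detach releases the character and stops ticking.
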(event `self.ReceiveTick`
  (params (DeltaSeconds :type "Float (single-precision)"))
  (`self.CameraStabilizer`))

(event `ToJETPACK`
  (bind (_returnvalue_x _returnvalue_y) (`KismetMathLibrary.BreakVector` (`self.K2_GetActorLocation` (`self.AsChar`))))
  (set `self.FollowPlayer` false)
  (bind (_direction _epicvetor _epicrotation) (`Timeline|TL_EpicRotation` :!label _label)
    (:`Update`
      (`self.K2_SetActorLocation` (`KismetMathLibrary.MakeVector` (+ _returnvalue_x (.x _epicvetor)) (+ _returnvalue_y (.y _epicvetor)) (.z _epicvetor)))
      (`SceneComponent.K2_SetRelativeRotation` (`self.Camera`) (`KismetMathLibrary.MakeRotator` 0.0 (.y _epicrotation) (.z _epicrotation)) false true))))

(event `CompleteToJETPACK`
  (bind (_returnvalue_x _returnvalue_y) (`KismetMathLibrary.BreakVector` (`self.K2_GetActorLocation` (`self.AsChar`))))
  (`|ExecutionSequence`
    (:`then_0`
      (goto _label :!via `Stop`))
    (:`then_1`
      (bind (_direction _epiclocation _epicrotation) (`Timeline|TL_CimpleteEpic`)
        (:`Update`
          (`self.K2_SetActorLocation` (`KismetMathLibrary.MakeVector` (+ _returnvalue_x (.x _epiclocation)) (+ _returnvalue_y (.y _epiclocation)) (.z _epiclocation)))
          (`SceneComponent.K2_SetRelativeRotation` (`self.Camera`) (`KismetMathLibrary.MakeRotator` 0.0 _epicrotation) false true))
        (:`Finished`
          (set `self.FollowPlayer` true)
          (`/Game/JamGame2023/Player/BP_PlayerChar.AddInputContext` (`self.AsChar`) "/Game/JamGame2023/Input/IMC_Jetpack.IMC_Jetpack" 0))))))

(fn `CameraStabilizer`
  (if (`self.FollowPlayer`)
    (bind _aschar (`self.AsChar`)
      (:`then`
        (if (`|EnumEquality` (`/Game/JamGame2023/Player/BP_PlayerChar.MovementState` _aschar) "NewEnumerator3")
          (bind _returnvalue_x (`KismetMathLibrary.BreakVector` (`self.K2_GetActorLocation` _aschar)))
          (`self.K2_SetActorLocation` (`KismetMathLibrary.MakeVector` (- _returnvalue_x 600.0) 0.0 450.0) false true)
          (else
            (bind _returnvalue_x_2 (`KismetMathLibrary.BreakVector` (`self.K2_GetActorLocation` _aschar)))
            (`self.K2_SetActorLocation` (`KismetMathLibrary.MakeVector` _returnvalue_x_2 800.0 215.0) false true))))
      (:`else`))))

(fn `Detach`
  (`self.K2_DetachFromActor` "KeepWorld" "KeepWorld" "KeepWorld")
  (set `self.AsChar` null)
  (`self.SetActorTickEnabled` false))

(fn `Setup`
  (params (Player :type "/Game/JamGame2023/Player/BP_PlayerChar Object Reference"))
  (set `self.AsChar` Player)
  (set `self.FollowPlayer` true)
  (`self.CameraStabilizer`)
  (`self.K2_AddActorWorldOffset` (200.0 0.0 0.0) false true)
  (set `self.FollowPlayer` false))

(fn `UserConstructionScript`)