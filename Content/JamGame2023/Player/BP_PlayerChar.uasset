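; Player pawn for an auto-runner with office and jetpack phases, owning game flow from main menu to end screen.
; Tick pushes it forward with manual gravity and ground projection via FloatingPawnMovement, while draining stamina at a rising rate until game over.
; Timeline jumps and timed, ceiling-checked slides can cancel into each other.
; ToJETPACK swaps input contexts, multiplies speed and drops gravity, with play-rate-scaled timelines stepping between horizontal and vertical lanes.
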(event `self.ReceiveBeginPlay`
  (bind _tl_horizontalmovement (`self.TL_HorizontalMovement`))
  (bind _tl_verticalmovement (`self.TL_VerticalMovement`))
  (bind _asplayer_controller (cast `PlayerController` (`self.GetController`) :!pure true))
  (set `self.Stamina` (`self.MaxStamina`))
  (bind _returnvalue (`|CreateWidget` "/Game/JamGame2023/UI/WBP_MainMenuWidget.WBP_MainMenuWidget_C" _asplayer_controller))
  (`/Game/JamGame2023/UI/WBP_MainMenuWidget.Setup` _returnvalue self)
  (`UserWidget.AddToViewport` _returnvalue 0)
  (`WidgetBlueprintLibrary.SetInputMode_GameAndUIEx` _asplayer_controller _returnvalue "DoNotLock" false)
  (set `PlayerController.bShowMouseCursor` true _asplayer_controller)
  (`TimelineComponent.SetPlaybackPosition` _tl_horizontalmovement 1.0 false true)
  (`TimelineComponent.SetPlayRate` _tl_horizontalmovement (/ (`self.JetManeuverSpeed`) (`self.HorizontalJetLineOffset`)))
  (`TimelineComponent.SetPlaybackPosition` _tl_verticalmovement 0.0 false true)
  (`TimelineComponent.SetPlayRate` _tl_verticalmovement (/ (`self.JetManeuverSpeed`) (`self.VerticalJetLineOffset`)))
  (bind _returnvalue_2 (`|SpawnActorFromClass` "/Game/JamGame2023/Player/BP_FollowingCamera.BP_FollowingCamera_C" (`KismetMathLibrary.MakeTransform` (0.0 0.0 0.0)) "Undefined" "MultiplyWithRoot" null null))
  (bind _output_get (set `self.FollowCamera` _returnvalue_2))
  (set `/Game/JamGame2023/Player/BP_FollowingCamera.AsChar` self _output_get)
  (bind _asbp_player_controller (cast `/Game/JamGame2023/Player/BP_PlayerController` (`self.GetController`)))
  (`PlayerController.SetViewTargetWithBlend` _asbp_player_controller (`self.FollowCamera`) 0.0 "VTBlend_Linear" 0.0 false))

(event `Start`
  (bind _asplayer_controller (cast `PlayerController` (`self.GetController`) :!pure true))
  (`self.AddInputContext` "/Game/JamGame2023/Input/IMC_Basic.IMC_Basic")
  (`self.AddInputContext` "/Game/JamGame2023/Input/IMC_Office.IMC_Office")
  (set `self.MovementState` "NewEnumerator0")
  (bind _returnvalue (`|CreateWidget` "/Game/JamGame2023/UI/WBP_MainPlayerWidget.WBP_MainPlayerWidget_C" _asplayer_controller))
  (`/Game/JamGame2023/UI/WBP_MainPlayerWidget.Setup` _returnvalue self)
  (`UserWidget.AddToViewport` _returnvalue 0)
  (`WidgetBlueprintLibrary.SetInputMode_GameOnly` _asplayer_controller true)
  (set `PlayerController.bShowMouseCursor` false _asplayer_controller)
  (`self.OnGameStart`))

(event `self.ReceiveTick`
  (params (DeltaSeconds :type "Float (single-precision)"))
  (if (`|EnumInequality` (`self.MovementState`) "NewEnumerator4")
    (`self.UpdateMovement` DeltaSeconds)
    (`self.DecayStamina` DeltaSeconds)
    (else
      (`MovementComponent.K2_MoveUpdatedComponent` :`self` (`self.FloatingPawnMovement`) :`Delta` (0.0 0.0 -10.0)))))

(event `EnhancedInput|/Game/JamGame2023/Input/IA_Jump`
  (params (ActionValue :type Boolean) (ElapsedSeconds :type "Float (double-precision)") (TriggeredSeconds :type "Float (double-precision)") (InputAction :type "InputAction Object Reference" :default "/Game/JamGame2023/Input/IA_Jump.IA_Jump"))
  (bind _movementstate (`self.MovementState`))
  (:`Triggered`
    (if (`|EnumEquality` _movementstate "NewEnumerator0")
      (set `self.MovementState` "NewEnumerator1" :!label _label)
      (bind (_direction _height) (`Timeline|TL_Jump` :!via `PlayFromStart`)
        (:`Update`
          (set `self.InputVector` (`KismetMathLibrary.MakeVector` 0.0 0.0 _height))
          (if (and (not (`self.InAir`)) (> (`TimelineComponent.GetPlaybackPosition` (`self.TL_Jump`)) 0.0))
            (`TimelineComponent.Stop` (`self.TL_Jump`))
            (set `self.InputVector` (0.0 0.0 0.0))
            (set `self.MovementState` "NewEnumerator0")
            (set `self.AllowBreakParcour` true))))
      (elif (and (`|EnumEquality` _movementstate "NewEnumerator2") (`self.AllowBreakParcour`))
        (set `self.AllowBreakParcour` false)
        (`KismetSystemLibrary.K2_ClearAndInvalidateTimerHandle` (`self.SlidingHandle`))
        (`SceneComponent.K2_SetRelativeLocation` (`self.Mesh`) (0.0 0.0 -88.0) false true)
        (`CapsuleComponent.SetCapsuleHalfHeight` (`self.Collision`) 88.0 true)
        (goto _label)))))

(event `EnhancedInput|/Game/JamGame2023/Input/IA_Slide`
  (params (ActionValue :type Boolean) (ElapsedSeconds :type "Float (double-precision)") (TriggeredSeconds :type "Float (double-precision)") (InputAction :type "InputAction Object Reference" :default "/Game/JamGame2023/Input/IA_Slide.IA_Slide"))
  (bind _movementstate (`self.MovementState`))
  (:`Triggered`
    (if (`|EnumEquality` _movementstate "NewEnumerator0")
      (set `self.MovementState` "NewEnumerator2" :!label _label_2)
      (`CapsuleComponent.SetCapsuleHalfHeight` (`self.Collision`) 30.0 true)
      (`SceneComponent.K2_SetRelativeLocation` (`self.Mesh`) (0.0 0.0 -36.0) false true)
      (bind _returnvalue (`KismetSystemLibrary.K2_SetTimerDelegate` (delegate `FinishSliding`) 0.54))
      (set `self.SlidingHandle` _returnvalue)
      (elif (and (`|EnumEquality` _movementstate "NewEnumerator1") (`self.AllowBreakParcour`))
        (set `self.AllowBreakParcour` false)
        (`TimelineComponent.Stop` (`self.TL_Jump`))
        (set `self.InputVector` (0.0 0.0 0.0))
        (goto _label_2)))))

(event `FinishSliding`
  (bind _returnvalue (`self.K2_GetActorLocation`))
  (bind (_outhit _returnvalue_2) (`KismetSystemLibrary.SphereTraceSingleForObjects` _returnvalue (+ _returnvalue (0.0 0.0 90.0)) 36.0 (`|MakeArray` "ObjectTypeQuery7" :!type "EObjectTypeQuery Enum")))
  (if _returnvalue_2
    (bind _returnvalue_3 (`KismetSystemLibrary.K2_SetTimerDelegate` (delegate `FinishSliding`) 0.05))
    (set `self.SlidingHandle` _returnvalue_3)
    (else
      (`SceneComponent.K2_SetRelativeLocation` (`self.Mesh`) (0.0 0.0 -88.0) false true)
      (`CapsuleComponent.SetCapsuleHalfHeight` (`self.Collision`) 88.0 true)
      (set `self.MovementState` "NewEnumerator0")
      (set `self.AllowBreakParcour` true))))

(event `self.Collision.OnComponentBeginOverlap`
  (params (OverlappedComponent :type "PrimitiveComponent Object Reference") (OtherActor :type "Actor Object Reference") (OtherComp :type "PrimitiveComponent Object Reference") (OtherBodyIndex :type Integer) (bFromSweep :type Boolean) (SweepResult :type "HitResult Structure (by ref)"))
  (bind _asbp_pickable_base (cast `/Game/JamGame2023/Pickups/BP_Pickable_Base` OtherActor)
    (:`then`
      (`/Game/JamGame2023/Pickups/BP_Pickable_Base.Collect` _asbp_pickable_base self))
    (:`CastFailed`
      (bind _asbp_obstacle_base (cast `/Game/JamGame2023/Obstacles/BP_Obstacle_Base` OtherActor))
      (`/Game/JamGame2023/Obstacles/BP_Obstacle_Base.Collide` _asbp_obstacle_base self))))

(event `EnhancedInput|/Game/JamGame2023/Input/IA_JetHorizontal`
  (params (ActionValue :type "Float (double-precision)") (ElapsedSeconds :type "Float (double-precision)") (TriggeredSeconds :type "Float (double-precision)") (InputAction :type "InputAction Object Reference" :default "/Game/JamGame2023/Input/IA_JetHorizontal.IA_JetHorizontal"))
  (bind (_returnvalue_x _returnvalue_y _returnvalue_z) (`KismetMathLibrary.BreakVector` (`self.K2_GetActorLocation`)))
  (:`Triggered`
    (if (`TimelineComponent.IsPlaying` (`self.TL_HorizontalMovement`))
      _
      (elif (> ActionValue 0.0)
        (bind (_direction _horizontalinput) (`Timeline|TL_HorizontalMovement` :!label _label_3)
          (:`Update`
            (`self.K2_SetActorLocation` (`KismetMathLibrary.MakeVector` _returnvalue_x (+ (* _horizontalinput (`self.HorizontalJetLineOffset`)) 0.0) _returnvalue_z) true))
          (:`PointReached`
            (goto _label_3 :!via `Stop`)))
        (else
          (goto _label_3 :!via `Reverse`))))))

(event `EnhancedInput|/Game/JamGame2023/Input/IA_JetVertical`
  (params (ActionValue :type "Float (double-precision)") (ElapsedSeconds :type "Float (double-precision)") (TriggeredSeconds :type "Float (double-precision)") (InputAction :type "InputAction Object Reference" :default "/Game/JamGame2023/Input/IA_JetVertical.IA_JetVertical"))
  (bind (_returnvalue_x _returnvalue_y) (`KismetMathLibrary.BreakVector` (`self.K2_GetActorLocation`)))
  (:`Triggered`
    (if (`TimelineComponent.IsPlaying` (`self.TL_VerticalMovement`))
      _
      (elif (> ActionValue 0.0)
        (bind (_direction _verticalinput) (`Timeline|TL_VerticalMovement` :!label _label_4)
          (:`Update`
            (`self.K2_SetActorLocation` (`KismetMathLibrary.MakeVector` _returnvalue_x _returnvalue_y (+ (* _verticalinput (`self.VerticalJetLineOffset`)) 100.0)) true))
          (:`PointReached`
            (goto _label_4 :!via `Stop`)))
        (else
          (goto _label_4 :!via `Reverse`))))))

(event `EnhancedInput|/Game/JamGame2023/Input/IA_Menu`
  (params (ActionValue :type Boolean) (ElapsedSeconds :type "Float (double-precision)") (TriggeredSeconds :type "Float (double-precision)") (InputAction :type "InputAction Object Reference" :default "/Game/JamGame2023/Input/IA_Menu.IA_Menu"))
  (bind _asplayer_controller (cast `PlayerController` (`self.GetController`) :!pure true))
  (:`Triggered`
    (bind _returnvalue (`GameplayStatics.SetGamePaused` true))
    (if _returnvalue
      (bind _returnvalue_2 (`|CreateWidget` "/Game/JamGame2023/UI/WBP_PauseMenu.WBP_PauseMenu_C" _asplayer_controller))
      (`UserWidget.AddToViewport` _returnvalue_2 0)
      (`WidgetBlueprintLibrary.SetInputMode_GameAndUIEx` _asplayer_controller _returnvalue_2 "DoNotLock" false)
      (set `PlayerController.bShowMouseCursor` true _asplayer_controller)
      (else
        (`/Game/JamGame2023/UI/WBP_PauseMenu.Continue` _returnvalue_2)))))

(fn `AddInputContext`
  (params (MappingContext :type "InputMappingContext Object Reference") (Priority :type Integer))
  (bind _asplayer_controller (cast `PlayerController` (`self.GetController`)))
  (`EnhancedInputSubsystemInterface.AddMappingContext` (pcsubsystem `EnhancedInputLocalPlayerSubsystem` _asplayer_controller) MappingContext Priority (make `ModifyContextOptions` true)))

(fn `AddStaminaDecayProtection`
  (params (AddedTime :type "Float (double-precision)"))
  (set `self.IgnoreStaminaDecay` (`KismetMathLibrary.FClamp` (+ (`self.IgnoreStaminaDecay`) AddedTime) 0.0 10.0)))

(fn `ChangeSpeed`
  (params (AddSpeed :type "Float (double-precision)"))
  (set `self.MovementSpeed` (+ AddSpeed (`self.MovementSpeed`))))

(fn `ChangeStamina`
  (params (StaminaDelta :type "Float (double-precision)"))
  (bind _output_get (set `self.Stamina` (`KismetMathLibrary.FClamp` (+ (`self.Stamina`) StaminaDelta) 0.0 (`self.MaxStamina`))))
  (if (<= _output_get 0.0)
    (`self.EndGame`)))

(fn `DecayStamina`
  (params (DeltaSeconds :type "Float (double-precision)"))
  (if (> (`self.IgnoreStaminaDecay`) 0.0)
    (set `self.IgnoreStaminaDecay` (- (`self.IgnoreStaminaDecay`) DeltaSeconds))
    (else
      (`self.ChangeStamina` (* DeltaSeconds (`self.StaminaDecay`) -1.0))))
  (set `self.StaminaDecay` (+ (`self.StaminaDecay`) (* (`self.StaminaDecayIncreaseRate`) (`local.DeltaSeconds`)))))

(fn `EndGame`
  (bind _asplayer_controller (cast `PlayerController` (`self.GetController`) :!pure true))
  (`self.OnGameOver`)
  (bind _returnvalue (`|CreateWidget` "/Game/JamGame2023/UI/WBP_EndScreen.WBP_EndScreen_C" _asplayer_controller))
  (`/Game/JamGame2023/UI/WBP_EndScreen.Setup` _returnvalue self)
  (`UserWidget.AddToViewport` _returnvalue 0)
  (`WidgetBlueprintLibrary.SetInputMode_GameAndUIEx` _asplayer_controller _returnvalue "DoNotLock" false)
  (set `PlayerController.bShowMouseCursor` true _asplayer_controller)
  (`/Game/JamGame2023/Player/BP_FollowingCamera.Detach` (`self.FollowCamera`))
  (`self.SetActorTickEnabled` false)
  (`self.SetActorHiddenInGame` true)
  (`SkeletalMeshComponent.SetAnimationMode` (`self.Mesh`) "AnimationCustomMode" true)
  (`AudioComponent.Stop` (`self.JetSound`)))

(fn `RemoveInputContext`
  (params (MappingContext :type "InputMappingContext Object Reference"))
  (bind _asplayer_controller (cast `PlayerController` (`self.GetController`)))
  (`EnhancedInputSubsystemInterface.RemoveMappingContext` (pcsubsystem `EnhancedInputLocalPlayerSubsystem` _asplayer_controller) MappingContext (make `ModifyContextOptions` true)))

(fn `ToJETPACK`
  (bind _returnvalue_x (`KismetMathLibrary.BreakVector` (`self.K2_GetActorLocation`)))
  (`self.RemoveInputContext` "/Game/JamGame2023/Input/IMC_Office.IMC_Office")
  (`SceneComponent.SetVisibility` (`self.Jetpack`) true false)
  (set `self.MovementState` "NewEnumerator3")
  (set `self.MovementSpeed` (* (`self.MovementSpeed`) (`self.JetpackSpeedMultoplier`)))
  (`KismetSystemLibrary.K2_ClearAndInvalidateTimerHandle` (`self.SlidingHandle`))
  (`TimelineComponent.Stop` (`self.TL_Jump`))
  (set `self.AllowBreakParcour` true)
  (set `self.InputVector` (0.0 0.0 0.0))
  (`SceneComponent.K2_SetRelativeLocation` (`self.Mesh`) (-55.0 0.0 -88.0) false true)
  (`self.K2_SetActorLocation` (`KismetMathLibrary.MakeVector` _returnvalue_x 0.0 100.0) false true)
  (`CapsuleComponent.SetCapsuleHalfHeight` (`self.Collision`) 36.0 true)
  (`self.AddInputContext` "/Game/JamGame2023/Input/IMC_Jetpack.IMC_Jetpack")
  (`/Game/JamGame2023/Player/BP_FollowingCamera.ToJETPACK` (`self.FollowCamera`))
  (`AudioComponent.Play` (`self.JetSound`) 0.0)
  (`self.OnJETPACK`))

(fn `UpdateMovement`
  (params (DeltaSeconds :type "Float (double-precision)"))
  (locals (L_Gravity :type "Vector Structure" :default (0.0 0.0 -980.0)) (L_TotalVector :type "Vector Structure"))
  (bind _output_get (set `local.L_TotalVector` (+ (* (1.0 0.0 0.0) (* DeltaSeconds (`self.MovementSpeed`))) (* (`self.InputVector`) (* DeltaSeconds (`self.ManeuverSpeed`))))))
  (bind _outhit (`MovementComponent.K2_MoveUpdatedComponent` :`self` (`self.FloatingPawnMovement`) :`Delta` (+ _output_get (`KismetMathLibrary.SelectVector` (* DeltaSeconds (`local.L_Gravity`)) (0.0 0.0 0.0) (`|EnumInequality` (`self.MovementState`) "NewEnumerator3")))))
  (bind (_bblockinghit _binitialoverlap _time _distance _location _impactpoint _normal _impactnormal) (`GameplayStatics.BreakHitResult` _outhit))
  (if (== _impactnormal (0.0 0.0 1.0))
    (set `self.InAir` false)
    (if (not (>= (.x _normal) 0.0))
      (set `local.L_TotalVector` (`KismetMathLibrary.ProjectVectorOnToPlane` (`local.L_TotalVector`) _normal)))
    (`MovementComponent.K2_MoveUpdatedComponent` :`self` (`self.FloatingPawnMovement`) :`Delta` (* (`local.L_TotalVector`) (- 1.0 _time)))
    (else
      (set `self.InAir` true))))

(fn `UserConstructionScript`
  (bind _jetpack (`self.Jetpack`))
  (`MeshComponent.SetVectorParameterValueOnMaterials` _jetpack "Color" (0.0 0.5 1.0))
  (`MeshComponent.SetScalarParameterValueOnMaterials` _jetpack "Roughness" 0.5))