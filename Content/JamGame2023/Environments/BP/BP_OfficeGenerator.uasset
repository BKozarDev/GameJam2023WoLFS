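; Generates a linear office level at BeginPlay as a row of BP_Background sections along X.
; Each section gets an obstacle by chance, picked by weighted random and rerolled to avoid repeating the previous class; the first gets BP_OfficeEmpty, the last BP_OfficeGlass.
; EnterArea destroys backgrounds behind the entered area and switches music at the second-to-last one.
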(event `ChangeMusic`
  (`KismetSystemLibrary.Delay` 0.8)
  (`AudioComponent.Stop` (`self.MS_MusicPart1`))
  (`AudioComponent.Play` (`self.MS_MusicPart2`) 0.0))

(event `self.ReceiveBeginPlay`
  (`self.SpawnBacks`)
  (`self.SpawnObstacles`))

(fn `EnterArea`
  (params (IndexArea :type Integer))
  (bind _output (`|GetArrayItem` (`self.SpawnBacksList`) (- IndexArea 3)))
  (if (> IndexArea 2)
    (if (!= IndexArea (- (`KismetArrayLibrary.Array_LastIndex` (`self.SpawnBacksList`)) 1))
      (if (`self.StartDeletingBackArea`)
        (`self.K2_DestroyActor` (`|GetArrayItem` (`self.SpawnBacksList`)))
        (set `self.StartDeletingBackArea` true)
        (else
          (`/Engine/EditorBlueprintResources/StandardMacros.IsValid` _output
            (:`Is Valid`
              (`self.K2_DestroyActor` _output)))))
      (else
        (`self.ChangeMusic`)))))

(fn `GetRandomObstacleClass`
  (returns (ActorClass :type "/Game/JamGame2023/Environments/BP/OfficeParts/BP_OfficePartsBase Class Reference"))
  (locals (L_RandomValue :type "Float (double-precision)") (L_ValueSum :type "Float (double-precision)"))
  (bind _keys (`BlueprintMapLibrary.Map_Keys` (`self.PartList`)))
  (for _array_element _keys
    (set `local.L_ValueSum` (+ (`BlueprintMapLibrary.Map_Find` (`self.PartList`) _array_element) (`local.L_ValueSum`))))
  (set `local.L_RandomValue` (`KismetMathLibrary.RandomFloatInRange` 0.0 (`local.L_ValueSum`)))
  (bind _keys_2 (`BlueprintMapLibrary.Map_Keys` (`self.PartList`)))
  (for _array_element_2 _keys_2
    (bind _value (`BlueprintMapLibrary.Map_Find` (`self.PartList`) _array_element_2))
    (if (< (`local.L_RandomValue`) _value)
      (return _array_element_2)
      (else
        (set `local.L_RandomValue` (- (`local.L_RandomValue`) _value))))))

(fn `SpawnBacks`
  (locals (L_SpawnCoords :type "Vector Structure" :default (0.0 0.0 0.0)) (L_SpawnActor :type "Actor Object Reference"))
  (bind (_returnvalue_x _returnvalue_y _returnvalue_z) (`KismetMathLibrary.BreakVector` (`self.K2_GetActorLocation`)))
  (bind _spawnbackslist (`self.SpawnBacksList`))
  (bind (_returnvalue_x_2 _returnvalue_y_2 _returnvalue_z_2) (`KismetMathLibrary.BreakVector` (`self.K2_GetActorLocation` (`|GetArrayItem` _spawnbackslist (`KismetArrayLibrary.Array_LastIndex` _spawnbackslist)))))
  (for _index (range (`self.PartsCount`))
    (if (== _index 0)
      (set `local.L_SpawnCoords` (`KismetMathLibrary.MakeVector` (+ (/ (`self.OffsetX`) 2.0) _returnvalue_x) _returnvalue_y _returnvalue_z))
      (else
        (set `local.L_SpawnCoords` (`KismetMathLibrary.MakeVector` (+ (`self.OffsetX`) _returnvalue_x_2) _returnvalue_y_2 _returnvalue_z_2))))
    (bind _returnvalue (`|SpawnActorFromClass` "/Game/JamGame2023/Environments/BP/OfficeParts/BP_Background.BP_Background_C" (`KismetMathLibrary.MakeTransform` (`local.L_SpawnCoords`) (struct :`Yaw` 90.0)) "Undefined" "MultiplyWithRoot" null _index null))
    (add `/Game/JamGame2023/Environments/BP/OfficeParts/BP_Background.OnEnterArea` _returnvalue (`|CreateDelegate` :!event `EnterArea`))
    (`KismetArrayLibrary.Array_Add` (`self.SpawnBacksList`) _returnvalue)))

(fn `SpawnObstacles`
  (for (_array_element _array_index) (`self.SpawnBacksList`)
    (if (!= _array_index 0)
      (if (!= _array_index (`KismetArrayLibrary.Array_LastIndex` (`self.SpawnBacksList`)))
        (if (<= (`KismetMathLibrary.RandomFloatInRange` 0.0 1.0) (`self.ObstacleChance`))
          (bind _actorclass (`self.GetRandomObstacleClass` :!label _label))
          (if (!= _actorclass (`GameplayStatics.GetObjectClass` (`self.PreviusObstacle`)))
            (bind _returnvalue (`|SpawnActorFromClass` _actorclass (`KismetMathLibrary.MakeTransform` (`SceneComponent.K2_GetComponentLocation` (`/Game/JamGame2023/Environments/BP/OfficeParts/BP_Background.GetSpawnPoint` _array_element))) "Undefined" "MultiplyWithRoot" null null))
            (`KismetArrayLibrary.Array_Add` (`self.SpawnObstacleList`) _returnvalue)
            (set `self.PreviusObstacle` _returnvalue)
            (else
              (goto _label))))
        (else
          (bind _returnvalue_2 (`|SpawnActorFromClass` "/Game/JamGame2023/Environments/BP/OfficeParts/BP_OfficeGlass.BP_OfficeGlass_C" (`KismetMathLibrary.MakeTransform` (`SceneComponent.K2_GetComponentLocation` (`/Game/JamGame2023/Environments/BP/OfficeParts/BP_Background.GetSpawnPoint` _array_element))) "Undefined" "MultiplyWithRoot" null null))
          (`KismetArrayLibrary.Array_Add` (`self.SpawnObstacleList`) _returnvalue_2)))
      (else
        (bind _returnvalue_3 (`|SpawnActorFromClass` "/Game/JamGame2023/Environments/BP/OfficeParts/BP_OfficeEmpty.BP_OfficeEmpty_C" (`KismetMathLibrary.MakeTransform` (`SceneComponent.K2_GetComponentLocation` (`/Game/JamGame2023/Environments/BP/OfficeParts/BP_Background.GetSpawnPoint` _array_element))) "Undefined" "MultiplyWithRoot" null null))
        (set `self.PreviusObstacle` _returnvalue_3)
        (`KismetArrayLibrary.Array_Add` (`self.SpawnObstacleList`) _returnvalue_3)))))

(fn `UserConstructionScript`)