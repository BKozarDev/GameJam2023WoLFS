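; BP_PickUpSpawner is a placeable spawn point that randomly creates a pickup at its location when play begins.
; On BeginPlay it rolls a random float against SpawnChance and, on success, spawns a random class from the PickUps array, then destroys itself.
; On a failed roll it spawns nothing and stays in the level.
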(event `self.ReceiveBeginPlay`
  (if (<= (`KismetMathLibrary.RandomFloatInRange` 0.0 1.0) (`self.SpawnChance`))
    (`|SpawnActorFromClass` (`|GetArrayItem` (`self.PickUps`) (`KismetMathLibrary.RandomInteger` (`KismetArrayLibrary.Array_Length` (`self.PickUps`)))) (`KismetMathLibrary.MakeTransform` (`self.K2_GetActorLocation`)) "Undefined" "MultiplyWithRoot" null null)
    (`self.K2_DestroyActor`)))

(fn `UserConstructionScript`)