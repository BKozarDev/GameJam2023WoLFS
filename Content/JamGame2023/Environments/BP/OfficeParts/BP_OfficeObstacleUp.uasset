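; BP_OfficeObstacleUp is an office obstacle, a lamp with point and spot lights, that penalizes the player on collision.
; Collide drains player stamina, runs the parent collide logic, plays a lamp-hit sound and calls Death.
; Death enables mesh physics with query-and-probe collision, removes both lights, then destroys the actor after a short delay.
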(event `Death`
  (bind _staticmesh (`self.StaticMesh`))
  (`PrimitiveComponent.SetSimulatePhysics` _staticmesh true)
  (`PrimitiveComponent.SetCollisionEnabled` _staticmesh "QueryAndProbe")
  (`ActorComponent.K2_DestroyComponent` (`self.PointLight`))
  (`ActorComponent.K2_DestroyComponent` (`self.SpotLight`))
  (`KismetSystemLibrary.Delay` 0.8)
  (`self.K2_DestroyActor`))

(event `self.ReceiveBeginPlay`)

(fn `Collide`
  (params (Player :type "/Game/JamGame2023/Player/BP_PlayerChar Object Reference"))
  (`/Game/JamGame2023/Player/BP_PlayerChar.ChangeStamina` Player -15.0)
  (`parent.Collide` Player)
  (`GameplayStatics.PlaySound2D` "/Game/Audio/SC_HitLamp.SC_HitLamp" 0.5 1.0 0.0 null null)
  (`self.Death`))

(fn `UserConstructionScript`)