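; BP_OfficeObstacleDown is an office obstacle that wipes out the player's stamina on collision.
; On BeginPlay it runs the parent logic, passes its vase, coffee cup and decor components to Init, and calls SpawnProps if that succeeds.
; Collide applies a huge negative stamina change to the player, then hands off to the parent's Collide.
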(event `self.ReceiveBeginPlay`
  (`parent.ReceiveBeginPlay`)
  (bind _isvalid (`self.Init` (`|MakeArray` (`self.SM_Vase_3`) (`self.SM_Coffee_cup_2`) (`self.SM_Coffee_cup`) (`self.SM_Decor_02`))))
  (if _isvalid
    (`self.Spawn Props`)))

(fn `Collide`
  (params (Player :type "/Game/JamGame2023/Player/BP_PlayerChar Object Reference"))
  (`/Game/JamGame2023/Player/BP_PlayerChar.ChangeStamina` Player -99999.0)
  (`parent.Collide` Player))

(fn `UserConstructionScript`
  (`parent.UserConstructionScript`))