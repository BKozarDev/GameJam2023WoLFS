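; BP_OfficeGlass is an office level piece that drives the player's jetpack sequence through three one-shot overlap triggers, each reacting only to BP_PlayerChar.
; Box switches the player to jetpack mode and hides the Jetpack mesh, JumpTrigger calls GoJump, and BreakTrigger calls CompleteJetting and plays a glass-break sound.
; The construction script tints the Jetpack material.
; A timeline for rotating the Jetpack exists but never runs.
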(event `self.Box.OnComponentBeginOverlap`
  (params (OverlappedComponent :type "PrimitiveComponent Object Reference") (OtherActor :type "Actor Object Reference") (OtherComp :type "PrimitiveComponent Object Reference") (OtherBodyIndex :type Integer) (bFromSweep :type Boolean) (SweepResult :type "HitResult Structure (by ref)"))
  (bind _asbp_player_char (cast `/Game/JamGame2023/Player/BP_PlayerChar` OtherActor))
  (`/Game/JamGame2023/Player/BP_PlayerChar.ToJETPACK` _asbp_player_char)
  (`PrimitiveComponent.SetCollisionEnabled` OverlappedComponent "NoCollision")
  (`SceneComponent.SetVisibility` (`self.Jetpack`) false false))

(event `CustomEvent`
  (`GameplayStatics.PlaySound2D` "/Game/Audio/Source/glassbreak.glassbreak" 1.0 1.0 0.12 null null :!label _label))

(event `self.BreakTrigger.OnComponentBeginOverlap`
  (params (OverlappedComponent :type "PrimitiveComponent Object Reference") (OtherActor :type "Actor Object Reference") (OtherComp :type "PrimitiveComponent Object Reference") (OtherBodyIndex :type Integer) (bFromSweep :type Boolean) (SweepResult :type "HitResult Structure (by ref)"))
  (bind _asbp_player_char (cast `/Game/JamGame2023/Player/BP_PlayerChar` OtherActor))
  (`PrimitiveComponent.SetCollisionEnabled` OverlappedComponent "NoCollision")
  (`/Game/JamGame2023/Player/BP_PlayerChar.CompleteJetting` _asbp_player_char)
  (goto _label))

(event `self.JumpTrigger.OnComponentBeginOverlap`
  (params (OverlappedComponent :type "PrimitiveComponent Object Reference") (OtherActor :type "Actor Object Reference") (OtherComp :type "PrimitiveComponent Object Reference") (OtherBodyIndex :type Integer) (bFromSweep :type Boolean) (SweepResult :type "HitResult Structure (by ref)"))
  (bind _asbp_player_char (cast `/Game/JamGame2023/Player/BP_PlayerChar` OtherActor))
  (`/Game/JamGame2023/Player/BP_PlayerChar.GoJump` _asbp_player_char)
  (`PrimitiveComponent.SetCollisionEnabled` OverlappedComponent "NoCollision"))

(fn `UserConstructionScript`
  (bind _jetpack (`self.Jetpack`))
  (`parent.UserConstructionScript`)
  (`MeshComponent.SetVectorParameterValueOnMaterials` _jetpack "Color" (0.0 0.5 1.0))
  (`MeshComponent.SetScalarParameterValueOnMaterials` _jetpack "Roughness" 0.5))