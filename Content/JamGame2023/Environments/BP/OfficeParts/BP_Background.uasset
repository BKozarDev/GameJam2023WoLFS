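; BP_Background is an office background segment that randomizes its look and serves as an area with an obstacle spawn point.
; On BeginPlay it shows one of two wall versions and one of six environment versions by toggling component visibility.
; Overlapping EnterCollision fires the OnEnterArea dispatcher with the segment's IndexArea.
; GetSpawnPoint exposes SpawnObstaclePoint to other code.
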(event `self.ReceiveBeginPlay`
  (bind _array (`|MakeArray` (`self.EnvVer1`) (`self.EnvVer2`) (`self.EnvVer3`) (`self.EnvVer4`) (`self.EnvVer5`) (`self.EnvVer6`)))
  (if (> (`KismetMathLibrary.RandomFloatInRange` 0.0 1.0) 0.5)
    (`SceneComponent.SetVisibility` (`self.WallVer1`) true true)
    (`SceneComponent.SetVisibility` (`self.WallVer2`) false true)
    (else
      (`SceneComponent.SetVisibility` (`self.WallVer2`) true true)
      (`SceneComponent.SetVisibility` (`self.WallVer1`) false true)))
  (for _array_element _array
    (`SceneComponent.SetVisibility` _array_element false true))
  (`SceneComponent.SetVisibility` (`|GetArrayItem` _array (`KismetMathLibrary.RandomInteger` (`KismetArrayLibrary.Array_Length` _array))) true true))

(event `self.EnterCollision.OnComponentBeginOverlap`
  (params (OverlappedComponent :type "PrimitiveComponent Object Reference") (OtherActor :type "Actor Object Reference") (OtherComp :type "PrimitiveComponent Object Reference") (OtherBodyIndex :type Integer) (bFromSweep :type Boolean) (SweepResult :type "HitResult Structure (by ref)"))
  (`self.OnEnterArea` (`self.IndexArea`)))

(fn `GetSpawnPoint`
  (returns (SpawnObstaclePoint :type "SceneComponent Object Reference"))
  (return (`self.SpawnObstaclePoint`)))

(fn `UserConstructionScript`)