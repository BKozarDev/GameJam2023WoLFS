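; Endless-runner spawner that fills the jet lines ahead of the player with obstacle and pickup waves along X.
; After a short delay it snaps to the player's FollowCamera, pre-generates 30 waves, then adds one each distance step.
; Each wave randomly fills six grid slots with long (sometimes tilted, blocking neighbors) or short obstacles, then tanks and rings in free slots.
; RemovingBox travels with it, destroying obstacles and pickables it overlaps.
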(event `self.ReceiveBeginPlay`
  (bind _accumulatedwaveoffset (`self.AccumulatedWaveOffset`))
  (`KismetSystemLibrary.Delay` 1.0)
  (bind _asbp_player_char (cast `/Game/JamGame2023/Player/BP_PlayerChar` (`Controller.K2_GetPawn` (`GameplayStatics.GetPlayerController` 0))))
  (bind _output_get (set `self.Player` _asbp_player_char))
  (`self.K2_AttachToActor` (`/Game/JamGame2023/Player/BP_PlayerChar.FollowCamera` _output_get) "None" "SnapToTarget" "SnapToTarget" "SnapToTarget")
  (for _ (range 30)
    (`self.GenerateWave` (+ _accumulatedwaveoffset (`self.StartWaveSpawnDistance`)))
    (set `self.AccumulatedWaveOffset` (+ _accumulatedwaveoffset (`self.WaveSpawnStep`))))
  (set `self.NextWaveThreshold` (`self.StartWaveSpawnDistance`)))

(event `self.ReceiveTick`
  (params (DeltaSeconds :type "Float (single-precision)"))
  (bind _returnvalue_x (`KismetMathLibrary.BreakVector` (`self.K2_GetActorLocation`)))
  (bind _accumulatedwaveoffset (`self.AccumulatedWaveOffset`))
  (bind _wavespawnstep (`self.WaveSpawnStep`))
  (if (>= _returnvalue_x (`self.NextWaveThreshold`))
    (`self.GenerateWave` (+ _accumulatedwaveoffset (`self.StartWaveSpawnDistance`)))
    (set `self.AccumulatedWaveOffset` (+ _accumulatedwaveoffset _wavespawnstep))
    (set `self.NextWaveThreshold` (+ (`self.NextWaveThreshold`) _wavespawnstep))))

(event `self.RemovingBox.OnComponentBeginOverlap`
  (params (OverlappedComponent :type "PrimitiveComponent Object Reference") (OtherActor :type "Actor Object Reference") (OtherComp :type "PrimitiveComponent Object Reference") (OtherBodyIndex :type Integer) (bFromSweep :type Boolean) (SweepResult :type "HitResult Structure (by ref)"))
  (bind _asbp_obstacle_base (cast `/Game/JamGame2023/Obstacles/BP_Obstacle_Base` OtherActor)
    (:`then`
      (`self.K2_DestroyActor` _asbp_obstacle_base))
    (:`CastFailed`
      (bind _asbp_pickable_base (cast `/Game/JamGame2023/Pickups/BP_Pickable_Base` OtherActor))
      (`self.K2_DestroyActor` _asbp_pickable_base))))

(fn `GenerateWave`
  (params (WaveX :type "Float (double-precision)"))
  (locals (L_OffsetsMap :type "Array of Vector Structure") (L_EmptySlots :type "Array of Integer") (L_SelectedSlot :type Integer) (L_SpawnTransform :type "Transform Structure") (L_Value :type Integer) (L_FValue :type "Float (double-precision)" :default 0.0))
  (bind _returnvalue (`KismetMathLibrary.MakeVector` WaveX 0.0 100.0))
  (bind (_horizontal _vertical) (`/Game/JamGame2023/Core/BPL_FuncLib.GetJetLineOffsets`))
  (bind _l_selectedslot (`local.L_SelectedSlot`))
  (bind _l_emptyslots (`local.L_EmptySlots`))
  (bind _l_emptyslots_2 (`local.L_EmptySlots`))
  (bind _l_emptyslots_3 (`local.L_EmptySlots`))
  (bind _l_emptyslots_4 (`local.L_EmptySlots`))
  (bind _l_emptyslots_5 (`local.L_EmptySlots`))
  (bind (_l_spawntransform_location _l_spawntransform_rotation _l_spawntransform_scale) (`KismetMathLibrary.BreakTransform` (`local.L_SpawnTransform`)))
  (bind _l_emptyslots_6 (`local.L_EmptySlots`))
  (bind _l_emptyslots_7 (`local.L_EmptySlots`))
  (bind _l_emptyslots_8 (`local.L_EmptySlots`))
  (bind _fewshorts_as1 (`self.FewShorts_As1`))
  (bind _l_emptyslots_9 (`local.L_EmptySlots`))
  (bind _l_emptyslots_10 (`local.L_EmptySlots`))
  (bind _singlelong (`self.SingleLong`))
  (bind _returnvalue_2 (<= (`KismetMathLibrary.RandomFloat`) 0.5))
  (bind _returnvalue_3 (+ _singlelong (`self.FewShorts`)))
  (bind _returnvalue_4 (* _horizontal -1.0))
  (bind _returnvalue_5 (+ _returnvalue (`KismetMathLibrary.MakeVector` 0.0 0.0 _vertical)))
  (set `local.L_OffsetsMap` (`|MakeArray` _returnvalue _returnvalue_5 (+ _returnvalue_5 (`KismetMathLibrary.MakeVector` 0.0 _returnvalue_4)) (+ _returnvalue_5 (`KismetMathLibrary.MakeVector` 0.0 _horizontal)) (+ _returnvalue (`KismetMathLibrary.MakeVector` 0.0 _returnvalue_4)) (+ _returnvalue (`KismetMathLibrary.MakeVector` 0.0 _horizontal))))
  (`|ExecutionSequence`
    (:`then_0`
      (bind _output_get (set `local.L_FValue` (`KismetMathLibrary.RandomFloat`)))
      (if (< _output_get _singlelong)
        (bind _output_get_2 (set `local.L_SelectedSlot` (`|GetArrayItem` _l_emptyslots_5 (`KismetMathLibrary.RandomInteger` (`KismetArrayLibrary.Array_Length` _l_emptyslots_5))) :!label _label))
        (`KismetArrayLibrary.Array_RemoveItem` _l_emptyslots_5 _output_get_2)
        (set `local.L_SpawnTransform` (`KismetMathLibrary.MakeTransform` (`|GetArrayItem` (`local.L_OffsetsMap`) _l_selectedslot) (struct :`Yaw` 180.0)))
        (switch `int` _l_selectedslot
          (:`0`
            (`KismetArrayLibrary.Array_RemoveItem` _l_emptyslots_6 4)
            (`KismetArrayLibrary.Array_RemoveItem` _l_emptyslots_6 5))
          (:`1`
            (`KismetArrayLibrary.Array_RemoveItem` _l_emptyslots_6 2)
            (`KismetArrayLibrary.Array_RemoveItem` _l_emptyslots_6 3))
          (:`2`
            (if _returnvalue_2
              (`KismetArrayLibrary.Array_RemoveItem` _l_emptyslots)
              (set `local.L_SpawnTransform` (`KismetMathLibrary.MakeTransform` _l_spawntransform_location (`KismetMathLibrary.ComposeRotators` _l_spawntransform_rotation (struct :`Roll` 30.0)) _l_spawntransform_scale) :!label _label_2)
              (else
                (`KismetArrayLibrary.Array_RemoveItem` _l_emptyslots 1))))
          (:`3`
            (if _returnvalue_2
              (`KismetArrayLibrary.Array_RemoveItem` _l_emptyslots_2)
              (set `local.L_SpawnTransform` (`KismetMathLibrary.MakeTransform` _l_spawntransform_location (`KismetMathLibrary.ComposeRotators` _l_spawntransform_rotation (struct :`Roll` -30.0)) _l_spawntransform_scale) :!label _label_3)
              (else
                (`KismetArrayLibrary.Array_RemoveItem` _l_emptyslots_2 1))))
          (:`4`
            (if _returnvalue_2
              (`KismetArrayLibrary.Array_RemoveItem` _l_emptyslots_3 1)
              (goto _label_3)
              (else
                (`KismetArrayLibrary.Array_RemoveItem` _l_emptyslots_3))))
          (:`5`
            (if _returnvalue_2
              (`KismetArrayLibrary.Array_RemoveItem` _l_emptyslots_4 1)
              (goto _label_2)
              (else
                (`KismetArrayLibrary.Array_RemoveItem` _l_emptyslots_4)))))
        (`|SpawnActorFromClass` "/Game/JamGame2023/Obstacles/JetObstacles/BP_JetLongObstacle.BP_JetLongObstacle_C" (`local.L_SpawnTransform`) "AlwaysSpawn" "MultiplyWithRoot" null null)
        (elif (< _output_get _returnvalue_3)
          (bind _output_get_3 (set `local.L_FValue` (`KismetMathLibrary.RandomFloat`)))
          (if (< _output_get_3 _fewshorts_as1)
            (set `local.L_Value` 0)
            (elif (< _output_get_3 (+ _fewshorts_as1 (`self.FewShorts_As2`)))
              (set `local.L_Value` 1)
              (else
                (set `local.L_Value` 2))))
          (for _ (range (+ (`local.L_Value`) 1))
            (bind _output_get_4 (set `local.L_SelectedSlot` (`|GetArrayItem` _l_emptyslots_8 (`KismetMathLibrary.RandomInteger` (`KismetArrayLibrary.Array_Length` _l_emptyslots_8)))))
            (`KismetArrayLibrary.Array_RemoveItem` (`local.L_EmptySlots`) _output_get_4)
            (`|SpawnActorFromClass` "/Game/JamGame2023/Obstacles/JetObstacles/BP_JetShortObstacle.BP_JetShortObstacle_C" (`KismetMathLibrary.MakeTransform` (`|GetArrayItem` (`local.L_OffsetsMap`) _output_get_4) (struct :`Yaw` 180.0)) "AlwaysSpawn" "MultiplyWithRoot" null null))
          (elif (< _output_get (+ _returnvalue_3 (`self.LongAndShorts`)))
            (`|ExecutionSequence`
              (:`then_0`
                (goto _label))
              (:`then_1`
                (if (< (`KismetMathLibrary.RandomFloat`) (`self.LongAndShorts_1Short`))
                  (set `local.L_Value` 0)
                  (else
                    (set `local.L_Value` 1)))
                (for _ (range (+ (`local.L_Value`) 1))
                  (bind _output_get_5 (set `local.L_SelectedSlot` (`|GetArrayItem` _l_emptyslots_7 (`KismetMathLibrary.RandomInteger` (`KismetArrayLibrary.Array_Length` _l_emptyslots_7)))))
                  (`KismetArrayLibrary.Array_RemoveItem` (`local.L_EmptySlots`) _output_get_5)
                  (`|SpawnActorFromClass` "/Game/JamGame2023/Obstacles/JetObstacles/BP_JetShortObstacle.BP_JetShortObstacle_C" (`KismetMathLibrary.MakeTransform` (`|GetArrayItem` (`local.L_OffsetsMap`) _output_get_5) (struct :`Yaw` 180.0)) "AlwaysSpawn" "MultiplyWithRoot" null null))))))))
    (:`then_1`
      (if (< (`KismetMathLibrary.RandomFloat`) (`self.Pickup`))
        (bind _output_get_6 (set `local.L_SelectedSlot` (`|GetArrayItem` _l_emptyslots_9 (`KismetMathLibrary.RandomInteger` (`KismetArrayLibrary.Array_Length` _l_emptyslots_9)))))
        (`|SpawnActorFromClass` "/Game/JamGame2023/Pickups/BP_Tank.BP_Tank_C" (`KismetMathLibrary.MakeTransform` (`|GetArrayItem` (`local.L_OffsetsMap`) _output_get_6) (struct)) "AlwaysSpawn" "MultiplyWithRoot" null null) ; Anyway just 1 variant
      )
      (bind _output_get_7 (set `local.L_FValue` (`KismetMathLibrary.RandomFloat`)))
      (if (< _output_get_7 0.1)
        (set `local.L_Value` 2)
        (for _ (range (+ (`local.L_Value`) 1)) :!label _label_4
          (if (`KismetArrayLibrary.Array_IsNotEmpty` (`local.L_EmptySlots`))
            (bind _output_get_8 (set `local.L_SelectedSlot` (`|GetArrayItem` _l_emptyslots_10 (`KismetMathLibrary.RandomInteger` (`KismetArrayLibrary.Array_Length` _l_emptyslots_10)))))
            (`KismetArrayLibrary.Array_RemoveItem` (`local.L_EmptySlots`) _output_get_8)
            (`|SpawnActorFromClass` "/Game/JamGame2023/Pickups/BP_Ring.BP_Ring_C" (`KismetMathLibrary.MakeTransform` (`|GetArrayItem` (`local.L_OffsetsMap`) _output_get_8)) "AlwaysSpawn" "MultiplyWithRoot" null null)))
        (elif (< _output_get_7 0.25)
          (set `local.L_Value` 1)
          (goto _label_4)
          (elif (< _output_get_7 0.6)
            (set `local.L_Value` 0)
            (goto _label_4)))))))

(fn `UserConstructionScript`)