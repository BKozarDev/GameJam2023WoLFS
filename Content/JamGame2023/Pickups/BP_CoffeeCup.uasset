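; BP_CoffeeCup is a coffee cup pickup that changes the collecting player's speed and stamina.
; Collect applies SpeedBonus and StaminaRecovery to the player, then hands off to the parent Collect.
; The construction script calls the parent's, then tints the mesh dark brown and sets its roughness through material parameters.
; A Rotation timeline maps its progression to a full yaw turn of the mesh, but nothing in the graph starts it.
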(fn `Collect`
  (params (Player :type "/Game/JamGame2023/Player/BP_PlayerChar Object Reference"))
  (`/Game/JamGame2023/Player/BP_PlayerChar.ChangeSpeed` Player (`self.SpeedBonus`))
  (`/Game/JamGame2023/Player/BP_PlayerChar.ChangeStamina` Player (`self.StaminaRecovery`))
  (`parent.Collect` Player))

(fn `UserConstructionScript`
  (bind _coffeecupmesh (`self.CoffeeCupMesh`))
  (`parent.UserConstructionScript`)
  (`MeshComponent.SetVectorParameterValueOnMaterials` _coffeecupmesh "Color" (0.16 0.07 0.0))
  (`MeshComponent.SetScalarParameterValueOnMaterials` _coffeecupmesh "Roughness" 0.68))