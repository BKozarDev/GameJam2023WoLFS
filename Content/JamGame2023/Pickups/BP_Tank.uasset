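; BP_Tank is a timed pickup that suspends the player's stamina decay for five seconds.
; Collect stores the player, turns on IgnoreStaminaDecay and starts a timer to EndBonus.
; EndBonus clears the flag and only then calls the parent Collect, so the base pickup logic is deferred until the bonus expires.
; A timeline for spinning the cylinder mesh is present but never triggered.
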(fn `Collect`
  (params (Player :type "/Game/JamGame2023/Player/BP_PlayerChar Object Reference"))
  (bind _output_get (set `self.Player` Player))
  (set `/Game/JamGame2023/Player/BP_PlayerChar.IgnoreStaminaDecay` true _output_get)
  (`KismetSystemLibrary.K2_SetTimer` null "EndBonus" 5.0))

(fn `EndBonus`
  (bind _player (`self.Player`))
  (set `/Game/JamGame2023/Player/BP_PlayerChar.IgnoreStaminaDecay` false _player)
  (`parent.Collect` _player))

(fn `UserConstructionScript`
  (`parent.UserConstructionScript`))