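; BP_Ring is a collectible ring pickup that boosts the player's speed and stamina.
; Its construction script creates one dynamic material, tints it pale yellow and shares it across the four cube meshes.
; On Collect, it disables collision to block repeat pickups, applies both boosts, turns the shared material green and plays a speed boost sound.
; It then hands off to the parent class's Collect.
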(fn `Collect`
  (params (Player :type "/Game/JamGame2023/Player/BP_PlayerChar Object Reference"))
  (`PrimitiveComponent.SetCollisionEnabled` (`self.Collision`) "NoCollision")
  (`/Game/JamGame2023/Player/BP_PlayerChar.ChangeSpeed` Player 50.0)
  (`/Game/JamGame2023/Player/BP_PlayerChar.ChangeStamina` Player 5.0)
  (`MaterialInstanceDynamic.SetVectorParameterValue` (`self.DynamicMat`) "Color" (struct :`R` 0.55 :`G` 1.0 :`A` 1.0))
  (`GameplayStatics.PlaySound2D` "/Game/Audio/Source/SpeedBoost.SpeedBoost" 1.0 1.0 0.0 null null)
  (`parent.Collect` Player))

(fn `UserConstructionScript`
  (`parent.UserConstructionScript`)
  (bind _returnvalue (`PrimitiveComponent.CreateDynamicMaterialInstance` (`self.Cube`) 0 null "None"))
  (bind _output_get (set `self.DynamicMat` _returnvalue))
  (`MaterialInstanceDynamic.SetVectorParameterValue` _output_get "Color" (struct :`R` 1.0 :`G` 0.939138 :`B` 0.677083 :`A` 1.0))
  (`MaterialInstanceDynamic.SetScalarParameterValue` _output_get "Roughness" 0.0)
  (`PrimitiveComponent.SetMaterial` (`self.Cube1`) 0 _output_get)
  (`PrimitiveComponent.SetMaterial` (`self.Cube3`) 0 _output_get)
  (`PrimitiveComponent.SetMaterial` (`self.Cube2`) 0 _output_get))