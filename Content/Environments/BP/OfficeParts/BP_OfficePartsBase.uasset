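; Base Blueprint for office environment parts that randomly varies which props are visible.
; Init stores a prop list, sets the base chance to one over its count, and reports whether the list had entries.
; SpawnProps toggles visibility on props that pass a roll, raising the chance after each miss and resetting it after a hit, so at least one gets toggled.
; Neither function is called within this Blueprint.
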(event `self.ReceiveBeginPlay`)

(fn `Init`
  (params (Props :type "Array of StaticMeshComponent Object Reference"))
  (returns (IsValid :type Boolean))
  (if (`KismetArrayLibrary.Array_IsEmpty` Props)
    (return false)
    (else
      (bind _output_get (set `self.PropsList` Props))
      (set `self.PropsSpawnRateBase` (/ 1.0 (`KismetMathLibrary.Conv_IntToDouble` (`KismetArrayLibrary.Array_Length` _output_get))))
      (return true))))

(fn `Spawn Props`
  (locals (L_SpawnChance :type "Float (double-precision)"))
  (set `local.L_SpawnChance` (`self.PropsSpawnRateBase`))
  (for _array_element (`self.PropsList`)
    (if (<= (`KismetMathLibrary.RandomFloatInRange` 0.0 1.0) (`local.L_SpawnChance`))
      (`SceneComponent.ToggleVisibility` _array_element true)
      (set `local.L_SpawnChance` (`self.PropsSpawnRateBase`))
      (else
        (set `local.L_SpawnChance` (+ (`local.L_SpawnChance`) (`self.PropsSpawnRateBase`)))))))

(fn `UserConstructionScript`)